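; Tripwire prop Blueprint that lays out two trip bars and a cable between them, with no active gameplay logic.
; The construction script offsets the second bar by BarEnd and yaws both bars using look-at rotations along their connecting line.
; It attaches the Wire to the first bar's WireSocket and sets its end location from the second bar's socket offset.
; The cable-length calculation is disconnected and never runs.
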(event EventBeginPlay)

(event Collision|EventActorBeginOverlap
  (params (OtherActor :type Actor%20Object%20Reference)))

(event EventTick
  (params (DeltaSeconds :type Float%20%28single-precision%29)))

(fn ConstructionScript
  (bind _trip_bar_02 (Variables|Default|Gettrip_bar_02))
  (bind _trip_bar_01 (Variables|Default|Gettrip_bar_01))
  (bind _trip_bar_02_2 (Variables|Default|Gettrip_bar_02))
  (bind _wire (Variables|Default|Getwire))
  (bind _trip_bar_01_2 (Variables|Default|Gettrip_bar_01))
  (bind _returnvalue (Transformation|GetWorldLocation _trip_bar_02))
  (bind _returnvalue_2 (Transformation|GetWorldLocation _trip_bar_01_2))
  (bind _returnvalue_3 (Math|Rotator|FindLookatRotation _returnvalue_2 _returnvalue))
  (bind _yaw (Math|Rotator|BreakRotator _returnvalue_3))
  (Transformation|AddRelativeLocation (Variables|Default|Gettrip_bar_02) (Variables|Default|GetBarEnd) false false)
  (Transformation|AddRelativeRotation _trip_bar_01 (Math|Rotator|MakeRotator 0.0 0.0 (+ _yaw 1.8e+02)) false false)
  (Transformation|AttachComponentToComponent _wire _trip_bar_01 "WireSocket" "KeepRelative" "KeepRelative" "KeepRelative" true)
  (Transformation|AddRelativeRotation _trip_bar_02_2 (Math|Rotator|MakeRotator 0.0 0.0 _yaw) false false)
  (Variables|/Script/CableComponent.CableComponent|SetEndLocation _wire (- (Transformation|GetSocketLocation _trip_bar_02_2 "WireSocket") (Transformation|GetWorldLocation _trip_bar_02_2))))